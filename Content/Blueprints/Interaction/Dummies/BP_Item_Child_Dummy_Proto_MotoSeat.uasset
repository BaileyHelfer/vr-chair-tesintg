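; Prototype drivable seat item, a child interaction dummy that is steered tank-style with two hand-grabbed sticks.
; BeginPlay registers three sub-components: a grabbable seat anchor and two X-constrained sticks that reset on release, whose rest positions are stored.
; Each Tick, the sticks' X offsets drive the actor, their sum moving it along local X and their difference yawing it.
; A separate event calls SitDown on the pawn with an attach reference.
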(event `self.ReceiveBeginPlay`
  (bind _man0scene2 (`self.Man0Scene2`))
  (`parent.ReceiveBeginPlay`)
  (`self.AddLogicToSubComponent` (`self.Man0Scene`) (`self.Man0Mesh`) (`self.Man0Highlighter`) (`self.Man0HandGhost`) null null (struct) (make `/Game/Blueprints/Helpers/Struct_GripOverrides` "NewEnumerator1" 1.0) (make `/Game/Blueprints/Helpers/Struct_SubOptions` true false true true true) (`|MakeArray` "None" :!type "Name"))
  (`self.AddLogicToSubComponent` (`self.Man0Scene1`) (`self.Man0Mesh1`) (`self.Man0Highlighter1`) (`self.Man0HandGhost1`) null null (make `/Game/Blueprints/Helpers/Struct_ConstraintContainer` "NewEnumerator1" (struct :`Speed` 10.0) (make `/Game/Blueprints/Helpers/Struct_LinearConstraints` "NewEnumerator3" 0.0 20.0 30.0) (struct :`BoundsType` "NewEnumerator0" :`ResetOnDrop?` true) (struct :`BoundsType` "NewEnumerator0" :`ResetOnDrop?` true) (struct :`BoundsType` "NewEnumerator0" :`HandAxisBinding` "NewEnumerator1" :`ResetOnDrop?` true) (struct :`BoundsType` "NewEnumerator0" :`HandAxisBinding` "NewEnumerator0" :`ResetOnDrop?` true) (struct :`BoundsType` "NewEnumerator0" :`HandAxisBinding` "NewEnumerator2" :`ResetOnDrop?` true)) (make `/Game/Blueprints/Helpers/Struct_GripOverrides` "NewEnumerator1" 1.0) (make `/Game/Blueprints/Helpers/Struct_SubOptions` true false false false true true) (`|MakeArray` "None" :!type "Name"))
  (set `self.RightStickCenter` (`SceneComponent.RelativeLocation` (`self.Man0Scene1`)))
  (`self.AddLogicToSubComponent` _man0scene2 (`self.Man0Mesh2`) (`self.Man0Highlighter2`) (`self.Man0HandGhost2`) null null (make `/Game/Blueprints/Helpers/Struct_ConstraintContainer` "NewEnumerator1" (struct :`Speed` 10.0) (make `/Game/Blueprints/Helpers/Struct_LinearConstraints` "NewEnumerator3" 0.0 20.0 30.0) (struct :`BoundsType` "NewEnumerator0" :`ResetOnDrop?` true) (struct :`BoundsType` "NewEnumerator0" :`ResetOnDrop?` true) (struct :`BoundsType` "NewEnumerator0" :`HandAxisBinding` "NewEnumerator1" :`ResetOnDrop?` true) (struct :`BoundsType` "NewEnumerator0" :`HandAxisBinding` "NewEnumerator0" :`ResetOnDrop?` true) (struct :`BoundsType` "NewEnumerator0" :`HandAxisBinding` "NewEnumerator2" :`ResetOnDrop?` true)) (make `/Game/Blueprints/Helpers/Struct_GripOverrides` "NewEnumerator1" 1.0) (make `/Game/Blueprints/Helpers/Struct_SubOptions` true false false false true true) (`|MakeArray` "None" :!type "Name"))
  (set `self.LeftStickCenter` (`SceneComponent.RelativeLocation` _man0scene2)))

(event `self.AttachPawnActorToSeat`
  (params (PawnActor :type "/Game/Blueprints/Pawn/BP_VR_Pawn Object Reference"))
  (`/Game/Blueprints/Pawn/BP_VR_Pawn.SitDown` PawnActor (`self.Attach1Ref`)))

(event `self.ReceiveTick`
  (params (DeltaSeconds :type "Float (single-precision)"))
  (bind _rightstickcenter_x (`KismetMathLibrary.BreakVector` (`self.RightStickCenter`)))
  (bind _leftstickcenter_x (`KismetMathLibrary.BreakVector` (`self.LeftStickCenter`)))
  (bind _relativelocation_x (`KismetMathLibrary.BreakVector` (`SceneComponent.RelativeLocation` (`self.Man0Scene1`))))
  (bind _relativelocation_x_2 (`KismetMathLibrary.BreakVector` (`SceneComponent.RelativeLocation` (`self.Man0Scene2`))))
  (`parent.ReceiveTick` DeltaSeconds)
  (`|ExecutionSequence`
    (:`then_0`
      (set `self.RightXDelta` (- _relativelocation_x _rightstickcenter_x))
      (set `self.LeftXDelta` (- _relativelocation_x_2 _leftstickcenter_x)))
    (:`then_1`
      (`self.K2_AddActorLocalRotation` (`KismetMathLibrary.MakeRotator` 0.0 0.0 (* (+ (* (`self.LeftXDelta`) (`self.RotMulti`)) (* (`self.RightXDelta`) -1.0 (`self.RotMulti`))) (`GameplayStatics.GetWorldDeltaSeconds`)))))
    (:`then_2`
      (`self.K2_AddActorLocalOffset` (`KismetMathLibrary.MakeVector` (* (+ (`self.LeftXDelta`) (`self.RightXDelta`)) (`GameplayStatics.GetWorldDeltaSeconds`) (`self.SpeedMulti`)))))))

(fn `UserConstructionScript`
  (`parent.UserConstructionScript`))